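; Self-replicating floor tile that builds endless ground around the ThirdPersonCharacter.
; On BeginPlay it reads the level number from BP_CheckChange and randomizes its 25 meshes from that level's background set.
; Player overlaps with trigger boxes spawn copies at sphere markers on sides and corners, skipping neighbours this tile already spawned.
; Leaving Sphere_delete destroys the tile, while entering Box4 triggers game over.
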(event `self.ReceiveBeginPlay`
  (bind _outactors (`GameplayStatics.GetAllActorsOfClass` "/Game/Kirill/BP_CheckChange.BP_CheckChange_C"))
  (bind _output (`|GetArrayItem` _outactors))
  (`/Engine/EditorBlueprintResources/StandardMacros.IsValid` _output
    (:`Is Valid`
      (set `self.nomer_lvl_pol` (`/Game/Kirill/BP_CheckChange.nomer_lvl` _output))
      (set `self.mesh` (`|MakeArray` (`self.Mesh13`) (`self.Mesh2`) (`self.Mesh3`) (`self.Mesh4`) (`self.Mesh5`) (`self.Mesh6`) (`self.Mesh7`) (`self.Mesh8`) (`self.Mesh9`) (`self.Mesh10`) (`self.Mesh11`) (`self.Mesh12`) (`self.Mesh1`) (`self.Mesh14`) (`self.Mesh15`) (`self.Mesh16`) (`self.Mesh17`) (`self.Mesh18`) (`self.Mesh19`) (`self.Mesh20`) (`self.Mesh21`) (`self.Mesh22`) (`self.Mesh23`) (`self.Mesh24`) (`self.Mesh25`)))
      (if (<= (`self.i_mesh`) 24) :!label _label
        ;[1 1 1] Меняем все меши на рандомные
        (`self.f_kakoi_mesh`)
        (`StaticMeshComponent.SetStaticMesh` (`|GetArrayItem` (`self.mesh`) (`self.i_mesh`)) (`self.new_mesh`))
        (set `self.i_mesh` (+ (`self.i_mesh`) 1))
        (goto _label)))
    (:`Is Not Valid`
      (`KismetSystemLibrary.PrintString` "999999"))))

(event `self.Box.OnComponentBeginOverlap`
  (params (OverlappedComponent :type "PrimitiveComponent Object Reference") (OtherActor :type "Actor Object Reference") (OtherComp :type "PrimitiveComponent Object Reference") (OtherBodyIndex :type Integer) (bFromSweep :type Boolean) (SweepResult :type "HitResult Structure (by ref)"))
  (bind _returnvalue_location (`KismetMathLibrary.BreakTransform` (`SceneComponent.K2_GetComponentToWorld` (`self.Sphere_pered`))))
  (bind _returnvalue_location_2 (`KismetMathLibrary.BreakTransform` (`SceneComponent.K2_GetComponentToWorld` (`self.Sphere_nasad`))))
  ;[1 1 1] Спавн новых блоков пола
  (cast `/Game/ThirdPersonBP/Blueprints/ThirdPersonCharacter` OtherActor)
  (`/Engine/EditorBlueprintResources/StandardMacros.IsValid` (`self.bp_pol1`) :!label _label_2
    (:`Is Valid`
      _)
    (:`Is Not Valid`
      (bind _returnvalue (`|SpawnActorFromClass` "BP_pol_1_C" (`KismetMathLibrary.MakeTransform` _returnvalue_location (`self.K2_GetActorRotation`) (`self.GetActorScale3D`)) "AlwaysSpawn" "OverrideRootScale" null null))
      (set `self.bp_pol1` _returnvalue)))
  (`/Engine/EditorBlueprintResources/StandardMacros.IsValid` (`self.bp_pol2`)
    (:`Is Not Valid`
      (bind _returnvalue_2 (`|SpawnActorFromClass` "BP_pol_1_C" (`KismetMathLibrary.MakeTransform` _returnvalue_location_2 (`self.K2_GetActorRotation`) (`self.GetActorScale3D`)) "AlwaysSpawn" "OverrideRootScale" null null))
      (set `self.bp_pol2` _returnvalue_2))))

(event `self.Box3.OnComponentBeginOverlap`
  (params (OverlappedComponent :type "PrimitiveComponent Object Reference") (OtherActor :type "Actor Object Reference") (OtherComp :type "PrimitiveComponent Object Reference") (OtherBodyIndex :type Integer) (bFromSweep :type Boolean) (SweepResult :type "HitResult Structure (by ref)"))
  ;[1 1 1] Спавн новых блоков пола
  (cast `/Game/ThirdPersonBP/Blueprints/ThirdPersonCharacter` OtherActor)
  (goto _label_2))

(event `self.Box4.OnComponentBeginOverlap`
  (params (OverlappedComponent :type "PrimitiveComponent Object Reference") (OtherActor :type "Actor Object Reference") (OtherComp :type "PrimitiveComponent Object Reference") (OtherBodyIndex :type Integer) (bFromSweep :type Boolean) (SweepResult :type "HitResult Structure (by ref)"))
  ;[1 1 1] Удаление игрока
  (bind _asthird_person_character (cast `/Game/ThirdPersonBP/Blueprints/ThirdPersonCharacter` OtherActor))
  (`/Game/ThirdPersonBP/Blueprints/ThirdPersonCharacter.Event_GameOver` _asthird_person_character))

(event `self.Box1.OnComponentBeginOverlap`
  (params (OverlappedComponent :type "PrimitiveComponent Object Reference") (OtherActor :type "Actor Object Reference") (OtherComp :type "PrimitiveComponent Object Reference") (OtherBodyIndex :type Integer) (bFromSweep :type Boolean) (SweepResult :type "HitResult Structure (by ref)"))
  (bind _returnvalue_location (`KismetMathLibrary.BreakTransform` (`SceneComponent.K2_GetComponentToWorld` (`self.Sphere_levo`))))
  (bind _returnvalue_location_2 (`KismetMathLibrary.BreakTransform` (`SceneComponent.K2_GetComponentToWorld` (`self.Sphere_pravo`))))
  ;[1 1 1] Спавн новых блоков пола
  (cast `/Game/ThirdPersonBP/Blueprints/ThirdPersonCharacter` OtherActor)
  (`/Engine/EditorBlueprintResources/StandardMacros.IsValid` (`self.bp_pol3`) :!label _label_3
    (:`Is Valid`
      _)
    (:`Is Not Valid`
      (bind _returnvalue (`|SpawnActorFromClass` "BP_pol_1_C" (`KismetMathLibrary.MakeTransform` _returnvalue_location_2 (`self.K2_GetActorRotation`) (`self.GetActorScale3D`)) "AlwaysSpawn" "OverrideRootScale" null null))
      (set `self.bp_pol3` _returnvalue)))
  (`/Engine/EditorBlueprintResources/StandardMacros.IsValid` (`self.bp_pol4`)
    (:`Is Not Valid`
      (bind _returnvalue_2 (`|SpawnActorFromClass` "BP_pol_1_C" (`KismetMathLibrary.MakeTransform` _returnvalue_location (`self.K2_GetActorRotation`) (`self.GetActorScale3D`)) "AlwaysSpawn" "OverrideRootScale" null null))
      (set `self.bp_pol4` _returnvalue_2))))

(event `self.sphere_delete.OnComponentEndOverlap`
  (params (OverlappedComponent :type "PrimitiveComponent Object Reference") (OtherActor :type "Actor Object Reference") (OtherComp :type "PrimitiveComponent Object Reference") (OtherBodyIndex :type Integer))
  ;[1 1 1] Удаление пола
  (cast `/Game/ThirdPersonBP/Blueprints/ThirdPersonCharacter` OtherActor)
  (`self.K2_DestroyActor`))

(event `self.Box2.OnComponentBeginOverlap`
  (params (OverlappedComponent :type "PrimitiveComponent Object Reference") (OtherActor :type "Actor Object Reference") (OtherComp :type "PrimitiveComponent Object Reference") (OtherBodyIndex :type Integer) (bFromSweep :type Boolean) (SweepResult :type "HitResult Structure (by ref)"))
  ;[1 1 1] Спавн новых блоков пола
  (cast `/Game/ThirdPersonBP/Blueprints/ThirdPersonCharacter` OtherActor)
  (goto _label_3))

(event `self.Box5.OnComponentBeginOverlap`
  (params (OverlappedComponent :type "PrimitiveComponent Object Reference") (OtherActor :type "Actor Object Reference") (OtherComp :type "PrimitiveComponent Object Reference") (OtherBodyIndex :type Integer) (bFromSweep :type Boolean) (SweepResult :type "HitResult Structure (by ref)"))
  (bind _returnvalue_location (`KismetMathLibrary.BreakTransform` (`SceneComponent.K2_GetComponentToWorld` (`self.Sphere_vpered_levo`))))
  ;[1 1 1] Спавн новых блоков пола по углам
  (cast `/Game/ThirdPersonBP/Blueprints/ThirdPersonCharacter` OtherActor)
  (`/Engine/EditorBlueprintResources/StandardMacros.IsValid` (`self.bp_pol_vpered_vlevo`)
    (:`Is Not Valid`
      (bind _returnvalue (`|SpawnActorFromClass` "BP_pol_1_C" (`KismetMathLibrary.MakeTransform` _returnvalue_location (`self.K2_GetActorRotation`) (`self.GetActorScale3D`)) "AlwaysSpawn" "OverrideRootScale" null null))
      (set `self.bp_pol_vpered_vlevo` _returnvalue))))

(event `self.Box8.OnComponentBeginOverlap`
  (params (OverlappedComponent :type "PrimitiveComponent Object Reference") (OtherActor :type "Actor Object Reference") (OtherComp :type "PrimitiveComponent Object Reference") (OtherBodyIndex :type Integer) (bFromSweep :type Boolean) (SweepResult :type "HitResult Structure (by ref)"))
  (bind _returnvalue_location (`KismetMathLibrary.BreakTransform` (`SceneComponent.K2_GetComponentToWorld` (`self.Sphere_vpered_pravo`))))
  ;[1 1 1] Спавн новых блоков пола по углам
  (cast `/Game/ThirdPersonBP/Blueprints/ThirdPersonCharacter` OtherActor)
  (`/Engine/EditorBlueprintResources/StandardMacros.IsValid` (`self.bp_pol_vpered_vpravo`)
    (:`Is Not Valid`
      (bind _returnvalue (`|SpawnActorFromClass` "BP_pol_1_C" (`KismetMathLibrary.MakeTransform` _returnvalue_location (`self.K2_GetActorRotation`) (`self.GetActorScale3D`)) "AlwaysSpawn" "OverrideRootScale" null null))
      (set `self.bp_pol_vpered_vpravo` _returnvalue))))

(event `self.Box9.OnComponentBeginOverlap`
  (params (OverlappedComponent :type "PrimitiveComponent Object Reference") (OtherActor :type "Actor Object Reference") (OtherComp :type "PrimitiveComponent Object Reference") (OtherBodyIndex :type Integer) (bFromSweep :type Boolean) (SweepResult :type "HitResult Structure (by ref)"))
  (bind _returnvalue_location (`KismetMathLibrary.BreakTransform` (`SceneComponent.K2_GetComponentToWorld` (`self.Sphere_nasad_vpravo`))))
  ;[1 1 1] Спавн новых блоков пола по углам
  (cast `/Game/ThirdPersonBP/Blueprints/ThirdPersonCharacter` OtherActor)
  (`/Engine/EditorBlueprintResources/StandardMacros.IsValid` (`self.bp_pol_nasad_vpravo`)
    (:`Is Not Valid`
      (bind _returnvalue (`|SpawnActorFromClass` "BP_pol_1_C" (`KismetMathLibrary.MakeTransform` _returnvalue_location (`self.K2_GetActorRotation`) (`self.GetActorScale3D`)) "AlwaysSpawn" "OverrideRootScale" null null))
      (set `self.bp_pol_nasad_vpravo` _returnvalue))))

(event `self.Box7.OnComponentBeginOverlap`
  (params (OverlappedComponent :type "PrimitiveComponent Object Reference") (OtherActor :type "Actor Object Reference") (OtherComp :type "PrimitiveComponent Object Reference") (OtherBodyIndex :type Integer) (bFromSweep :type Boolean) (SweepResult :type "HitResult Structure (by ref)"))
  (bind _returnvalue_location (`KismetMathLibrary.BreakTransform` (`SceneComponent.K2_GetComponentToWorld` (`self.Sphere_nasad_vlevo`))))
  ;[1 1 1] Спавн новых блоков пола по углам
  (cast `/Game/ThirdPersonBP/Blueprints/ThirdPersonCharacter` OtherActor)
  (`/Engine/EditorBlueprintResources/StandardMacros.IsValid` (`self.bp_pol_nasad_vlevo`)
    (:`Is Not Valid`
      (bind _returnvalue (`|SpawnActorFromClass` "BP_pol_1_C" (`KismetMathLibrary.MakeTransform` _returnvalue_location (`self.K2_GetActorRotation`) (`self.GetActorScale3D`)) "AlwaysSpawn" "OverrideRootScale" null null))
      (set `self.bp_pol_nasad_vlevo` _returnvalue))))

(fn `f_kakoi_mesh`
  (switch `string` (`KismetStringLibrary.Conv_IntToString` (`self.nomer_lvl_pol`))
    (:`1`
      (switch `string` (`KismetStringLibrary.Conv_IntToString` (`KismetMathLibrary.FTrunc` (`KismetMathLibrary.RandomFloatInRange` 1.0 6.0)))
        (:`1`
          (set `self.new_mesh` "/Game/Kirill/Assets/Geometry/Merged_Background_Fire/SM_F_Background_V1.SM_F_Background_V1"))
        (:`2`
          (set `self.new_mesh` "/Game/Kirill/Assets/Geometry/Merged_Background_Fire/SM_F_Background_V2.SM_F_Background_V2"))
        (:`3`
          (set `self.new_mesh` "/Game/Kirill/Assets/Geometry/Merged_Background_Fire/SM__F_Background_V3.SM__F_Background_V3"))
        (:`4`
          (set `self.new_mesh` "/Game/Kirill/Assets/Geometry/Merged_Background_Fire/SM_F_Background_V4.SM_F_Background_V4"))
        (:`5`
          (set `self.new_mesh` "/Game/Kirill/Assets/Geometry/Merged_Background_Fire/SM_F_Background_V5.SM_F_Background_V5"))
        (:`6`
          (set `self.new_mesh` "/Game/Kirill/Assets/Geometry/Merged_Background_Fire/SM_F_Background_V6.SM_F_Background_V6"))))
    (:`2`
      (switch `string` (`KismetStringLibrary.Conv_IntToString` (`KismetMathLibrary.FTrunc` (`KismetMathLibrary.RandomFloatInRange` 1.0 6.0)))
        (:`1`
          (set `self.new_mesh` "/Game/Kirill/Assets/Geometry/Merged_Background_Radiation/SM_R_Background_V1.SM_R_Background_V1"))
        (:`2`
          (set `self.new_mesh` "/Game/Kirill/Assets/Geometry/Merged_Background_Radiation/SM_R_Background_V2.SM_R_Background_V2"))
        (:`3`
          (set `self.new_mesh` "/Game/Kirill/Assets/Geometry/Merged_Background_Radiation/SM_R_Background_V3.SM_R_Background_V3"))
        (:`4`
          (set `self.new_mesh` "/Game/Kirill/Assets/Geometry/Merged_Background_Radiation/SM_R_Background_V4.SM_R_Background_V4"))
        (:`5`
          (set `self.new_mesh` "/Game/Kirill/Assets/Geometry/Merged_Background_Radiation/SM_R_Background_V5.SM_R_Background_V5"))
        (:`6`
          (set `self.new_mesh` "/Game/Kirill/Assets/Geometry/Merged_Background_Radiation/SM_R_Background_V6.SM_R_Background_V6"))))
    (:`3`
      (switch `string` (`KismetStringLibrary.Conv_IntToString` (`KismetMathLibrary.FTrunc` (`KismetMathLibrary.RandomFloatInRange` 1.0 6.0)))
        (:`1`
          (set `self.new_mesh` "/Game/Kirill/Assets/Geometry/Merged_Backgroung_Water/SM_W_Background_V1.SM_W_Background_V1"))
        (:`2`
          (set `self.new_mesh` "/Game/Kirill/Assets/Geometry/Merged_Backgroung_Water/SM_W_Background_V2.SM_W_Background_V2"))
        (:`3`
          (set `self.new_mesh` "/Game/Kirill/Assets/Geometry/Merged_Backgroung_Water/SM_W_Background_V3.SM_W_Background_V3"))
        (:`4`
          (set `self.new_mesh` "/Game/Kirill/Assets/Geometry/Merged_Backgroung_Water/SM_W_Background_V4.SM_W_Background_V4"))
        (:`5`
          (set `self.new_mesh` "/Game/Kirill/Assets/Geometry/Merged_Backgroung_Water/SM_W_Background_V5.SM_W_Background_V5"))
        (:`6`
          (set `self.new_mesh` "/Game/Kirill/Assets/Geometry/Merged_Backgroung_Water/SM_W_Background_V6.SM_W_Background_V6"))))))

(fn `UserConstructionScript`)