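; Self-chaining landscape platform that procedurally extends the player's path and scatters obstacles on itself.
; BeginPlay picks a level-specific factory class from BP_CheckChange's level number and usually spawns jittered obstacles at three points, randomizing the class only before the middle one.
; The trigger box spawns, once, that factory or another platform, straight or via a right-turn piece; left turns are disconnected.
; Leaving the sphere destroys platform and obstacles after a delay.
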(event `Event_spawn`
  ;[1 1 1] Спавн препятствий
  (`self.f_spawn_pregrada` (`self.z_location_spawn`) (`self.sphere_prepjatstvie`))
  (if (and (`KismetMathLibrary.RandomBool`) (`self.spawn_dva?`))
    (`self.f_spawn_pregrada` (`self.z_location_spawn`) (`self.sphere_prepjatstvie`))
    (if (`KismetMathLibrary.RandomBool`)
      (`self.f_spawn_pregrada` (`self.z_location_spawn`) (`self.sphere_prepjatstvie`))
      (if (`KismetMathLibrary.RandomBool`)
        (`self.f_spawn_pregrada` (`self.z_location_spawn`) (`self.sphere_prepjatstvie`))))))

(event `Event_spawn_2`
  ;[1 1 1] Спавн препятствий
  (`self.f_spawn_pregrada` (`self.z_location_spawn`) (`self.sphere_prepjatstvie1`))
  (if (and (`KismetMathLibrary.RandomBool`) (`self.spawn_dva?`))
    (`self.f_spawn_pregrada` (`self.z_location_spawn`) (`self.sphere_prepjatstvie1`))
    (if (`KismetMathLibrary.RandomBool`)
      (`self.f_spawn_pregrada` (`self.z_location_spawn`) (`self.sphere_prepjatstvie1`))
      (if (`KismetMathLibrary.RandomBool`)
        (`self.f_spawn_pregrada` (`self.z_location_spawn`) (`self.sphere_prepjatstvie1`))))))

(event `Event_spawn_3`
  ;[1 1 1] Спавн препятствий
  (`self.f_spawn_pregrada` (`self.z_location_spawn`) (`self.sphere_prepjatstvie2`))
  (if (and (`KismetMathLibrary.RandomBool`) (`self.spawn_dva?`))
    (`self.f_spawn_pregrada` (`self.z_location_spawn`) (`self.sphere_prepjatstvie2`))
    (if (`KismetMathLibrary.RandomBool`)
      (`self.f_spawn_pregrada` (`self.z_location_spawn`) (`self.sphere_prepjatstvie2`))
      (if (`KismetMathLibrary.RandomBool`)
        (`self.f_spawn_pregrada` (`self.z_location_spawn`) (`self.sphere_prepjatstvie2`))))))

(event `self.ReceiveBeginPlay`
  (bind _outactors (`GameplayStatics.GetAllActorsOfClass` "/Game/Kirill/BP_CheckChange.BP_CheckChange_C"))
  (set `self.nomer_lvl` (`/Game/Kirill/BP_CheckChange.nomer_lvl` (`|GetArrayItem` _outactors)))
  (`self.f_kotel`)
  ;[1 1 1] Вероятность появления препятствия
  (bind _output_get (set `self.i_prepjatstvie` (`KismetMathLibrary.RandomFloatInRange` 1.0 100.0)))
  (if (<= _output_get 90.0)
    (`self.Event_spawn`)
    (`self.Event_spawn_3`)
    ;[1 1 1] Определение какие предметы заспавнятся
    (bind _output_get_2 (set `self.i_element` (`KismetMathLibrary.FTrunc` (`KismetMathLibrary.RandomFloatInRange` 2.0 4.0))))
    (switch `string` (`KismetStringLibrary.Conv_IntToString` _output_get_2)
      (:`2`
        (set `self.bp_abstracte_element_class` (`self.bp_botschka`))
        (set `self.z_location_spawn` 30.0))
      (:`3`
        (set `self.bp_abstracte_element_class` (`self.bp_truba`))
        (set `self.spawn_dva?` false))
      (:`4`
        (set `self.bp_abstracte_element_class` (`self.bp_object1`))
        (set `self.z_location_spawn` 600.0)))
    (bind _output_get_3 (set `self.i_element` (`KismetMathLibrary.FTrunc` (`KismetMathLibrary.RandomFloatInRange` 2.0 4.0))))
    (switch `string` (`KismetStringLibrary.Conv_IntToString` _output_get_3)
      (:`2`
        (set `self.bp_abstracte_element_class` (`self.bp_botschka`))
        (set `self.z_location_spawn` 30.0))
      (:`3`
        (set `self.bp_abstracte_element_class` (`self.bp_truba`))
        (set `self.spawn_dva?` false))
      (:`4`
        (set `self.bp_abstracte_element_class` (`self.bp_object1`))
        (set `self.z_location_spawn` 600.0)))
    (`self.Event_spawn_2`)))

(event `self.Box_spawn.OnComponentBeginOverlap`
  (params (OverlappedComponent :type "PrimitiveComponent Object Reference") (OtherActor :type "Actor Object Reference") (OtherComp :type "PrimitiveComponent Object Reference") (OtherBodyIndex :type Integer) (bFromSweep :type Boolean) (SweepResult :type "HitResult Structure (by ref)"))
  (bind _returnvalue (`SceneComponent.K2_GetComponentToWorld` (`self.sphere_krai_pravo`)))
  (bind _returnvalue_2 (`SceneComponent.K2_GetComponentToWorld` (`self.sphere_spawn_pravo`)))
  (bind _returnvalue_3 (`SceneComponent.K2_GetComponentToWorld` (`self.spawn_zavod`)))
  (bind _returnvalue_4 (`SceneComponent.K2_GetComponentToWorld` (`self.sphere_krai_centr`)))
  (cast `/Game/ThirdPersonBP/Blueprints/ThirdPersonCharacter` OtherActor)
  (if (`self.active?`)
    (bind _output_get (set `self.i_zavod` (`KismetMathLibrary.RandomFloatInRange` 1.0 100.0)))
    (if (< _output_get 40.0)
      ;[1 1 1] Спавн завода
      (`|SpawnActorFromClass` (`self.bp_kotel_lvl`) (`KismetMathLibrary.MakeTransform` (.location _returnvalue_3) (`KismetMathLibrary.MakeRotator` (.roll (.rotation _returnvalue_3)) (.pitch (.rotation _returnvalue_3)) (.yaw (.rotation _returnvalue_3))) (`self.GetActorScale3D`)) "AlwaysSpawn" "OverrideRootScale" null null)
      (else
        ;[1 1 1] Спавн новых блоков
        (bind _output_get_2 (set `self.i_napravlenie` (`KismetMathLibrary.RandomFloatInRange` 1.0 100.0)))
        (if (<= _output_get_2 40.0)
          (`|SpawnActorFromClass` "BP_landschaft_C" (`KismetMathLibrary.MakeTransform` (.location _returnvalue_4) (`KismetMathLibrary.MakeRotator` 0.0 0.0 (.yaw (.rotation _returnvalue_4))) (`self.GetActorScale3D`)) "AlwaysSpawn" "OverrideRootScale" null null)
          (else
            (if (<= (`self.i_napravlenie`) 70.0)
              _
              (else
                _))
            (bind _returnvalue_5 (`|SpawnActorFromClass` "/Game/Kirill/BP_povorot_platformi_2.BP_povorot_platformi_2_C" (`KismetMathLibrary.MakeTransform` (.location _returnvalue) (`KismetMathLibrary.MakeRotator` 0.0 0.0 (+ (.yaw (.rotation _returnvalue)) 90.0)) (0.825 0.825 1.0)) "AlwaysSpawn" "OverrideRootScale" null null))
            (set `self.bp_platforma_1` _returnvalue_5)
            (`|SpawnActorFromClass` "BP_landschaft_C" (`KismetMathLibrary.MakeTransform` (.location _returnvalue_2) (`KismetMathLibrary.MakeRotator` 0.0 0.0 (+ (.yaw (.rotation _returnvalue_2)) 45.0)) (`self.GetActorScale3D`)) "AlwaysSpawn" "OverrideRootScale" null null)))
        (set `self.active?` false)))))

(event `self.Sphere.OnComponentEndOverlap`
  (params (OverlappedComponent :type "PrimitiveComponent Object Reference") (OtherActor :type "Actor Object Reference") (OtherComp :type "PrimitiveComponent Object Reference") (OtherBodyIndex :type Integer))
  (bind _bp_pregrada (`self.bp_pregrada`))
  ;[1 1 1] Удаление платформы
  (cast `/Game/ThirdPersonBP/Blueprints/ThirdPersonCharacter` OtherActor)
  (`KismetSystemLibrary.Delay` 1.0)
  (`/Engine/EditorBlueprintResources/StandardMacros.IsValid` (`|GetArrayItem` _bp_pregrada)
    (:`Is Valid`
      (`self.K2_DestroyActor` _bp_pregrada))
    (:`Is Not Valid`
      _))
  (`self.K2_DestroyActor` self))

(fn `f_kotel`
  (switch `string` (`KismetStringLibrary.Conv_IntToString` (`self.nomer_lvl`))
    (:`1`
      (set `self.bp_kotel_lvl` "/Game/Kirill/Assets/Blueprints/Kotel/BP_Fuel.BP_Fuel_C"))
    (:`2`
      (set `self.bp_kotel_lvl` "/Game/Kirill/Assets/Blueprints/Kotel/BP_Kotel.BP_Kotel_C"))
    (:`3`
      (set `self.bp_kotel_lvl` "/Game/Kirill/Assets/Blueprints/Kotel/BP_Water.BP_Water_C"))))

(fn `f_spawn_pregrada`
  (params (z :type "Float (double-precision)") (component :type "SphereComponent Object Reference"))
  (bind _returnvalue (`SceneComponent.K2_GetComponentToWorld` component))
  (bind _returnvalue_2 (`|SpawnActorFromClass` (`self.bp_abstracte_element_class`) (`KismetMathLibrary.MakeTransform` (+ (.location _returnvalue) (`KismetMathLibrary.MakeVector` (`KismetMathLibrary.RandomFloatInRange` -200.0 200.0) (`KismetMathLibrary.RandomFloatInRange` -200.0 200.0) z)) (`KismetMathLibrary.MakeRotator` 0.0 0.0 (.yaw (.rotation _returnvalue))) (`self.GetActorScale3D`)) "AdjustIfPossibleButAlwaysSpawn" "OverrideRootScale" null null))
  (`KismetArrayLibrary.Array_Add` (`self.bp_pregrada`) _returnvalue_2))

(fn `f_spawn_pregrada_2`
  (params (z :type "Float (double-precision)"))
  (returns (NewParam :type "/Game/Kirill/BP_abstract_element Object Reference"))
  (bind _returnvalue (`SceneComponent.K2_GetComponentToWorld` (`self.sphere_prepjatstvie1`)))
  (bind _returnvalue_2 (`|SpawnActorFromClass` (`self.bp_abstracte_element_class`) (`KismetMathLibrary.MakeTransform` (+ (.location _returnvalue) (`KismetMathLibrary.MakeVector` (`KismetMathLibrary.RandomFloatInRange` -200.0 200.0) (`KismetMathLibrary.RandomFloatInRange` -200.0 200.0) z)) (`KismetMathLibrary.MakeRotator` 0.0 0.0 (.yaw (.rotation _returnvalue))) (`self.GetActorScale3D`)) "AdjustIfPossibleButAlwaysSpawn" "OverrideRootScale" null null))
  (return _returnvalue_2))

(fn `f_spawn_pregrada_3`
  (params (z :type "Float (double-precision)"))
  (returns (NewParam :type "/Game/Kirill/BP_abstract_element Object Reference"))
  (bind _returnvalue (`SceneComponent.K2_GetComponentToWorld` (`self.sphere_prepjatstvie1`)))
  (bind _returnvalue_2 (`|SpawnActorFromClass` (`self.bp_abstracte_element_class`) (`KismetMathLibrary.MakeTransform` (+ (.location _returnvalue) (`KismetMathLibrary.MakeVector` (`KismetMathLibrary.RandomFloatInRange` -200.0 200.0) (`KismetMathLibrary.RandomFloatInRange` -200.0 200.0) z)) (`KismetMathLibrary.MakeRotator` 0.0 0.0 (.yaw (.rotation _returnvalue))) (`self.GetActorScale3D`)) "AdjustIfPossibleButAlwaysSpawn" "OverrideRootScale" null null))
  (return _returnvalue_2))

(fn `UserConstructionScript`)