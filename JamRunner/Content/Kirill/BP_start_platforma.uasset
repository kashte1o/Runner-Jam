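; BP_start_platforma is the starting platform, destroyed 10 seconds after ThirdPersonCharacter leaves Sphere1.
; Helper functions, never called here, spawn randomly offset obstacles, pick a boiler/fuel/water class by level number, and randomly spawn forward or lever pipe modules, storing spawned actors in arrays.
; Lever variant selection tests random floats for exact equality, so it almost always yields V4.
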(event `self.ReceiveBeginPlay`)

(event `self.Sphere1.OnComponentEndOverlap`
  (params (OverlappedComponent :type "PrimitiveComponent Object Reference") (OtherActor :type "Actor Object Reference") (OtherComp :type "PrimitiveComponent Object Reference") (OtherBodyIndex :type Integer))
  ;[1 1 1] Удаление платформы при старте
  (cast `/Game/ThirdPersonBP/Blueprints/ThirdPersonCharacter` OtherActor)
  (`KismetSystemLibrary.Delay` 10.0)
  (`self.K2_DestroyActor`))

(fn `f_kotel`
  (switch `string` (`KismetStringLibrary.Conv_IntToString` (`self.nomer_lvl`))
    (:`1`
      (set `self.bp_kotel_lvl` "/Game/Kirill/Assets/Blueprints/Kotel/BP_Fuel.BP_Fuel_C"))
    (:`2`
      (set `self.bp_kotel_lvl` "/Game/Kirill/Assets/Blueprints/Kotel/BP_Kotel.BP_Kotel_C"))
    (:`3`
      (set `self.bp_kotel_lvl` "/Game/Kirill/Assets/Blueprints/Kotel/BP_Water.BP_Water_C"))))

(fn `f_spawn_object`
  (params (sphere :type "SphereComponent Object Reference"))
  (bind _returnvalue (`KismetMathLibrary.RandomFloatInRange` 1.0 4.0))
  (bind _returnvalue_2 (`SceneComponent.K2_GetComponentToWorld` sphere))
  (bind _returnvalue_3 (`SceneComponent.K2_GetComponentToWorld` sphere))
  (if (< (`KismetMathLibrary.RandomFloatInRange` 1.0 100.0) 10.0)
    (bind _returnvalue_4 (`|SpawnActorFromClass` "/Game/Kirill/Assets/Blueprints/Truba/BP_Truba_Module_Forward.BP_Truba_Module_Forward_C" (`KismetMathLibrary.MakeTransform` (+ (.location _returnvalue_3) (0.0 0.0 350.0)) (`KismetMathLibrary.MakeRotator` 0.0 0.0 (- (.yaw (.rotation _returnvalue_3)) 90.0)) (`self.GetActorScale3D`)) "Undefined" "OverrideRootScale" null null))
    (`KismetArrayLibrary.Array_Add` (`self.BP_Truba_Module_Forward`) _returnvalue_4)
    (else
      (if (== _returnvalue 1.0)
        (set `self.bp_trub` "/Game/Kirill/Assets/Blueprints/Rychag/BP_Truba_Module_Rychag_V1.BP_Truba_Module_Rychag_V1_C")
        (elif (== _returnvalue 2.0)
          (set `self.bp_trub` "/Game/Kirill/Assets/Blueprints/Rychag/BP_Truba_Module_Rychag_V2.BP_Truba_Module_Rychag_V2_C")
          (elif (== _returnvalue 3.0)
            (set `self.bp_trub` "/Game/Kirill/Assets/Blueprints/Rychag/BP_Truba_Module_Rychag_V3.BP_Truba_Module_Rychag_V3_C")
            (else
              (set `self.bp_trub` "/Game/Kirill/Assets/Blueprints/Rychag/BP_Truba_Module_Rychag_V4.BP_Truba_Module_Rychag_V4_C")))))
      (if (< (`KismetMathLibrary.RandomFloatInRange` 1.0 100.0) 15.0)
        (bind _returnvalue_5 (`|SpawnActorFromClass` (`self.bp_trub`) (`KismetMathLibrary.MakeTransform` (+ (.location _returnvalue_2) (0.0 0.0 350.0)) (`KismetMathLibrary.MakeRotator` 0.0 0.0 (- (.yaw (.rotation _returnvalue_2)) 90.0)) (`self.GetActorScale3D`)) "Undefined" "OverrideRootScale" null null))
        (`KismetArrayLibrary.Array_Add` (`self.BP_Truba_Module_Rychag`) _returnvalue_5)))))

(fn `f_spawn_pregrada`
  (params (z :type "Float (double-precision)") (component :type "SphereComponent Object Reference"))
  (bind _returnvalue (`SceneComponent.K2_GetComponentToWorld` component))
  (bind _returnvalue_2 (`|SpawnActorFromClass` (`self.bp_abstracte_element_class`) (`KismetMathLibrary.MakeTransform` (+ (.location _returnvalue) (`KismetMathLibrary.MakeVector` (`KismetMathLibrary.RandomFloatInRange` -200.0 200.0) (`KismetMathLibrary.RandomFloatInRange` -200.0 200.0) z)) (`KismetMathLibrary.MakeRotator` 0.0 0.0 (.yaw (.rotation _returnvalue))) (`self.GetActorScale3D`)) "AdjustIfPossibleButAlwaysSpawn" "OverrideRootScale" null null))
  (`KismetArrayLibrary.Array_Add` (`self.bp_pregrada`) _returnvalue_2))

(fn `UserConstructionScript`)