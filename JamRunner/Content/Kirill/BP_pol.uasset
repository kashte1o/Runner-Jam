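; BP_pol is a self-replicating level piece that spawns more copies of itself as the ThirdPersonCharacter moves through it.
; Two trigger boxes each spawn a pair of copies at their own two sphere component transforms, ignoring collisions.
; Stored references to the copies block respawning while either of that pair still exists.
; Each copy carries the same triggers, so the layout can keep growing; nothing here destroys pieces.
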(event `self.Box.OnComponentBeginOverlap`
  (params (OverlappedComponent :type "PrimitiveComponent Object Reference") (OtherActor :type "Actor Object Reference") (OtherComp :type "PrimitiveComponent Object Reference") (OtherBodyIndex :type Integer) (bFromSweep :type Boolean) (SweepResult :type "HitResult Structure (by ref)"))
  (cast `/Game/ThirdPersonBP/Blueprints/ThirdPersonCharacter` OtherActor)
  (`/Engine/EditorBlueprintResources/StandardMacros.IsValid` (`self.bp_pol1`)
    (:`Is Not Valid`
      (`/Engine/EditorBlueprintResources/StandardMacros.IsValid` (`self.bp_pol2`)
        (:`Is Not Valid`
          (bind _returnvalue (`|SpawnActorFromClass` "BP_pol_C" (`SceneComponent.K2_GetComponentToWorld` (`self.Sphere2`)) "AlwaysSpawn" "OverrideRootScale" null null))
          (set `self.bp_pol1` _returnvalue)
          (bind _returnvalue_2 (`|SpawnActorFromClass` "BP_pol_C" (`SceneComponent.K2_GetComponentToWorld` (`self.Sphere3`)) "AlwaysSpawn" "OverrideRootScale" null null))
          (set `self.bp_pol2` _returnvalue_2))))))

(event `self.Box1.OnComponentBeginOverlap`
  (params (OverlappedComponent :type "PrimitiveComponent Object Reference") (OtherActor :type "Actor Object Reference") (OtherComp :type "PrimitiveComponent Object Reference") (OtherBodyIndex :type Integer) (bFromSweep :type Boolean) (SweepResult :type "HitResult Structure (by ref)"))
  (cast `/Game/ThirdPersonBP/Blueprints/ThirdPersonCharacter` OtherActor)
  (`/Engine/EditorBlueprintResources/StandardMacros.IsValid` (`self.bp_pol3`)
    (:`Is Not Valid`
      (`/Engine/EditorBlueprintResources/StandardMacros.IsValid` (`self.bp_pol4`)
        (:`Is Not Valid`
          (bind _returnvalue (`|SpawnActorFromClass` "BP_pol_C" (`SceneComponent.K2_GetComponentToWorld` (`self.Sphere`)) "AlwaysSpawn" "OverrideRootScale" null null))
          (set `self.bp_pol3` _returnvalue)
          (bind _returnvalue_2 (`|SpawnActorFromClass` "BP_pol_C" (`SceneComponent.K2_GetComponentToWorld` (`self.Sphere1`)) "AlwaysSpawn" "OverrideRootScale" null null))
          (set `self.bp_pol4` _returnvalue_2))))))

(fn `UserConstructionScript`)