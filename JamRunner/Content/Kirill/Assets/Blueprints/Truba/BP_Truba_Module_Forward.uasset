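; Truba module Blueprint for a forward piece that varies its look by picking a random tile mesh when play begins.
; BeginPlay truncates a random float to an integer, stores it in IElement and switches on its string form to set the Module static mesh to one of four variants.
; Because the float range tops out at the last index, truncation makes the fourth variant almost never appear.
; The construction script only calls its parent.
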(event `self.ReceiveBeginPlay`
  (bind _module (`self.Module`))
  (bind _output_get (set `self.i_element` (`KismetMathLibrary.FTrunc` (`KismetMathLibrary.RandomFloatInRange` 1.0 4.0))))
  (switch `string` (`KismetStringLibrary.Conv_IntToString` _output_get)
    (:`1`
      (`StaticMeshComponent.SetStaticMesh` _module "/Game/Kirill/Assets/Geometry/SM_MERGED_Truba_Tile_V1.SM_MERGED_Truba_Tile_V1"))
    (:`2`
      (`StaticMeshComponent.SetStaticMesh` _module "/Game/Kirill/Assets/Geometry/SM_MERGED_Truba_Tile_V2.SM_MERGED_Truba_Tile_V2"))
    (:`3`
      (`StaticMeshComponent.SetStaticMesh` _module "/Game/Kirill/Assets/Geometry/SM_MERGED_Truba_Tile_V3.SM_MERGED_Truba_Tile_V3"))
    (:`4`
      (`StaticMeshComponent.SetStaticMesh` _module "/Game/Kirill/Assets/Geometry/SM_MERGED_Truba_Tile_V4.SM_MERGED_Truba_Tile_V4"))))

(fn `UserConstructionScript`
  (`parent.UserConstructionScript`))