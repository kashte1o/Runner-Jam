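; BP_Colba is an actor with a Colba component that breaks into a splash when its sphere is overlapped.
; On overlap it destroys Colba and plays a timeline that uniformly scales SMSplash.
; A short delay, started from the timeline's update, then destroys the actor.
; A second timeline meant to loop a yaw rotation on Colba is unconnected and never runs.
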(event `self.Sphere.OnComponentBeginOverlap`
  (params (OverlappedComponent :type "PrimitiveComponent Object Reference") (OtherActor :type "Actor Object Reference") (OtherComp :type "PrimitiveComponent Object Reference") (OtherBodyIndex :type Integer) (bFromSweep :type Boolean) (SweepResult :type "HitResult Structure (by ref)"))
  (`ActorComponent.K2_DestroyComponent` (`self.Colba`))
  (bind (_direction _newtrack_0) (`Timeline|Timeline_1`)
    (:`Update`
      (`SceneComponent.SetRelativeScale3D` (`self.SM_Splash`) (`KismetMathLibrary.MakeVector` _newtrack_0 _newtrack_0 _newtrack_0))
      (`KismetSystemLibrary.Delay` 0.3)
      (`self.K2_DestroyActor`))))

(fn `UserConstructionScript`)