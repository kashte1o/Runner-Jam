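; Fuel actor that animates the roll of four upper truss (FermaVerh) meshes toward 90 degrees.
; BeginPlay starts one timeline per mesh, and overlapping that mesh's collision component replays its timeline from the start.
; Each update lerps from the mesh's current roll rather than a stored start value, so the motion compounds instead of following the curve directly.
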(event `self.ReceiveBeginPlay`
  (bind _sm_ferma_verh_03 (`self.SM_Ferma_Verh_03`))
  (bind _sm_ferma_verh_04 (`self.SM_Ferma_Verh_04`))
  (bind _sm_ferma_verh_01 (`self.SM_Ferma_Verh_01`))
  (bind _sm_ferma_verh_02 (`self.SM_Ferma_Verh_02`))
  (bind (_relativerotation_roll _relativerotation_pitch _relativerotation_yaw) (`KismetMathLibrary.BreakRotator` (`SceneComponent.RelativeRotation` _sm_ferma_verh_04)))
  (bind (_relativerotation_roll_2 _relativerotation_pitch_2 _relativerotation_yaw_2) (`KismetMathLibrary.BreakRotator` (`SceneComponent.RelativeRotation` _sm_ferma_verh_01)))
  (bind (_relativerotation_roll_3 _relativerotation_pitch_3 _relativerotation_yaw_3) (`KismetMathLibrary.BreakRotator` (`SceneComponent.RelativeRotation` _sm_ferma_verh_02)))
  (bind (_relativerotation_roll_4 _relativerotation_pitch_4 _relativerotation_yaw_4) (`KismetMathLibrary.BreakRotator` (`SceneComponent.RelativeRotation` _sm_ferma_verh_03)))
  (`|ExecutionSequence`
    (:`then_0`
      (bind (_direction _newtrack_0) (`Timeline|Timeline_0` :!label _label)
        (:`Update`
          (`SceneComponent.K2_SetRelativeRotation` _sm_ferma_verh_01 (`KismetMathLibrary.MakeRotator` (`KismetMathLibrary.Lerp` _relativerotation_roll_2 90.0 _newtrack_0) _relativerotation_pitch_2 _relativerotation_yaw_2) false false))))
    (:`then_1`
      (bind (_direction_2 _newtrack_0_2) (`Timeline|Timeline_1` :!label _label_2)
        (:`Update`
          (`SceneComponent.K2_SetRelativeRotation` _sm_ferma_verh_02 (`KismetMathLibrary.MakeRotator` (`KismetMathLibrary.Lerp` _relativerotation_roll_3 90.0 _newtrack_0_2) _relativerotation_pitch_3 _relativerotation_yaw_3) false false))))
    (:`then_2`
      (bind (_direction_3 _newtrack_0_3) (`Timeline|Timeline_2` :!label _label_3)
        (:`Update`
          (`SceneComponent.K2_SetRelativeRotation` _sm_ferma_verh_03 (`KismetMathLibrary.MakeRotator` (`KismetMathLibrary.Lerp` _relativerotation_roll_4 90.0 _newtrack_0_3) _relativerotation_pitch_4 _relativerotation_yaw_4) false false))))
    (:`then_3`
      (bind (_direction_4 _newtrack_0_4) (`Timeline|Timeline_3` :!label _label_4)
        (:`Update`
          (`SceneComponent.K2_SetRelativeRotation` _sm_ferma_verh_04 (`KismetMathLibrary.MakeRotator` (`KismetMathLibrary.Lerp` _relativerotation_roll 90.0 _newtrack_0_4) _relativerotation_pitch _relativerotation_yaw) false false))))))

(event `self.Collision_1.OnComponentBeginOverlap`
  (params (OverlappedComponent :type "PrimitiveComponent Object Reference") (OtherActor :type "Actor Object Reference") (OtherComp :type "PrimitiveComponent Object Reference") (OtherBodyIndex :type Integer) (bFromSweep :type Boolean) (SweepResult :type "HitResult Structure (by ref)"))
  (goto _label :!via `PlayFromStart`))

(event `self.Collision_2.OnComponentBeginOverlap`
  (params (OverlappedComponent :type "PrimitiveComponent Object Reference") (OtherActor :type "Actor Object Reference") (OtherComp :type "PrimitiveComponent Object Reference") (OtherBodyIndex :type Integer) (bFromSweep :type Boolean) (SweepResult :type "HitResult Structure (by ref)"))
  (goto _label_2 :!via `PlayFromStart`))

(event `self.Collision_3.OnComponentBeginOverlap`
  (params (OverlappedComponent :type "PrimitiveComponent Object Reference") (OtherActor :type "Actor Object Reference") (OtherComp :type "PrimitiveComponent Object Reference") (OtherBodyIndex :type Integer) (bFromSweep :type Boolean) (SweepResult :type "HitResult Structure (by ref)"))
  (goto _label_3 :!via `PlayFromStart`))

(event `self.Collision_4.OnComponentBeginOverlap`
  (params (OverlappedComponent :type "PrimitiveComponent Object Reference") (OtherActor :type "Actor Object Reference") (OtherComp :type "PrimitiveComponent Object Reference") (OtherBodyIndex :type Integer) (bFromSweep :type Boolean) (SweepResult :type "HitResult Structure (by ref)"))
  (goto _label_4 :!via `PlayFromStart`))

(fn `UserConstructionScript`)