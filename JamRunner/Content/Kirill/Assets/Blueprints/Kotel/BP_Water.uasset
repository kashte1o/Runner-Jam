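; BP_Water is a level piece that spawns a BP_landschaft actor at its SpawnDoroga transform on BeginPlay, using its own scale.
; Four collision components each play a timeline when ThirdPersonCharacter overlaps them, rotating the matching SMFermaVerh mesh toward 90 degrees roll.
; Each update lerps from the mesh's current roll rather than a stored start value.
; Three timelines that would lower the water meshes are unconnected and never run.
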(event `self.ReceiveBeginPlay`
  (bind _returnvalue (`SceneComponent.K2_GetComponentToWorld` (`self.spawn_doroga`)))
  (`|SpawnActorFromClass` "/Game/Kirill/BP_landschaft.BP_landschaft_C" (`KismetMathLibrary.MakeTransform` (.location _returnvalue) (`KismetMathLibrary.MakeRotator` 0.0 0.0 (.yaw (.rotation _returnvalue))) (`self.GetActorScale3D`)) "AlwaysSpawn" "OverrideRootScale" null null))

(event `self.Collision_5.OnComponentBeginOverlap`
  (params (OverlappedComponent :type "PrimitiveComponent Object Reference") (OtherActor :type "Actor Object Reference") (OtherComp :type "PrimitiveComponent Object Reference") (OtherBodyIndex :type Integer) (bFromSweep :type Boolean) (SweepResult :type "HitResult Structure (by ref)"))
  (bind _sm_ferma_verh_01 (`self.SM_Ferma_Verh_01`))
  (bind (_relativerotation_roll _relativerotation_pitch _relativerotation_yaw) (`KismetMathLibrary.BreakRotator` (`SceneComponent.RelativeRotation` _sm_ferma_verh_01)))
  (cast `/Game/ThirdPersonBP/Blueprints/ThirdPersonCharacter` OtherActor)
  (bind (_direction _newtrack_0) (`Timeline|Timeline_0` :!via `PlayFromStart`)
    (:`Update`
      (`SceneComponent.K2_SetRelativeRotation` _sm_ferma_verh_01 (`KismetMathLibrary.MakeRotator` (`KismetMathLibrary.Lerp` _relativerotation_roll 90.0 _newtrack_0) _relativerotation_pitch _relativerotation_yaw) false false))))

(event `CustomEvent_0`)

(event `self.Collision_6.OnComponentBeginOverlap`
  (params (OverlappedComponent :type "PrimitiveComponent Object Reference") (OtherActor :type "Actor Object Reference") (OtherComp :type "PrimitiveComponent Object Reference") (OtherBodyIndex :type Integer) (bFromSweep :type Boolean) (SweepResult :type "HitResult Structure (by ref)"))
  (bind _sm_ferma_verh_02 (`self.SM_Ferma_Verh_02`))
  (bind (_relativerotation_roll _relativerotation_pitch _relativerotation_yaw) (`KismetMathLibrary.BreakRotator` (`SceneComponent.RelativeRotation` _sm_ferma_verh_02)))
  (cast `/Game/ThirdPersonBP/Blueprints/ThirdPersonCharacter` OtherActor)
  (bind (_direction _newtrack_0) (`Timeline|Timeline_1` :!via `PlayFromStart`)
    (:`Update`
      (`SceneComponent.K2_SetRelativeRotation` _sm_ferma_verh_02 (`KismetMathLibrary.MakeRotator` (`KismetMathLibrary.Lerp` _relativerotation_roll 90.0 _newtrack_0) _relativerotation_pitch _relativerotation_yaw) false false))))

(event `self.Collision_7.OnComponentBeginOverlap`
  (params (OverlappedComponent :type "PrimitiveComponent Object Reference") (OtherActor :type "Actor Object Reference") (OtherComp :type "PrimitiveComponent Object Reference") (OtherBodyIndex :type Integer) (bFromSweep :type Boolean) (SweepResult :type "HitResult Structure (by ref)"))
  (bind _sm_ferma_verh_03 (`self.SM_Ferma_Verh_03`))
  (bind (_relativerotation_roll _relativerotation_pitch _relativerotation_yaw) (`KismetMathLibrary.BreakRotator` (`SceneComponent.RelativeRotation` _sm_ferma_verh_03)))
  (cast `/Game/ThirdPersonBP/Blueprints/ThirdPersonCharacter` OtherActor)
  (bind (_direction _newtrack_0) (`Timeline|Timeline_2` :!via `PlayFromStart`)
    (:`Update`
      (`SceneComponent.K2_SetRelativeRotation` _sm_ferma_verh_03 (`KismetMathLibrary.MakeRotator` (`KismetMathLibrary.Lerp` _relativerotation_roll 90.0 _newtrack_0) _relativerotation_pitch _relativerotation_yaw) false false))))

(event `self.Collision_8.OnComponentBeginOverlap`
  (params (OverlappedComponent :type "PrimitiveComponent Object Reference") (OtherActor :type "Actor Object Reference") (OtherComp :type "PrimitiveComponent Object Reference") (OtherBodyIndex :type Integer) (bFromSweep :type Boolean) (SweepResult :type "HitResult Structure (by ref)"))
  (bind _sm_ferma_verh_04 (`self.SM_Ferma_Verh_04`))
  (bind (_relativerotation_roll _relativerotation_pitch _relativerotation_yaw) (`KismetMathLibrary.BreakRotator` (`SceneComponent.RelativeRotation` _sm_ferma_verh_04)))
  (cast `/Game/ThirdPersonBP/Blueprints/ThirdPersonCharacter` OtherActor)
  (bind (_direction _newtrack_0) (`Timeline|Timeline_3` :!via `PlayFromStart`)
    (:`Update`
      (`SceneComponent.K2_SetRelativeRotation` _sm_ferma_verh_04 (`KismetMathLibrary.MakeRotator` (`KismetMathLibrary.Lerp` _relativerotation_roll 90.0 _newtrack_0) _relativerotation_pitch _relativerotation_yaw) false false))))

(fn `UserConstructionScript`)