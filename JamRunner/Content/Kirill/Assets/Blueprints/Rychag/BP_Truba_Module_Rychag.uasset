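; Pipe module actor (lever set) whose box trigger sends the player into a video cutscene and on to ThirdPersonExampleMap.
; On character overlap it calls the scale event, zeroes speed and shows a W_CutScene widget with the Green_lights playlist.
; It clears StartGame on the game instance and opens the map after a fixed delay, while video end separately removes the widget.
; Unconnected logic for level-based buffs and level selection never runs.
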(event `self.Box.OnComponentBeginOverlap`
  (params (OverlappedComponent :type "PrimitiveComponent Object Reference") (OtherActor :type "Actor Object Reference") (OtherComp :type "PrimitiveComponent Object Reference") (OtherBodyIndex :type Integer) (bFromSweep :type Boolean) (SweepResult :type "HitResult Structure (by ref)"))
  (bind _media_player (`self.Media Player`))
  (bind _asthird_person_character (cast `/Game/ThirdPersonBP/Blueprints/ThirdPersonCharacter` OtherActor))
  (`/Game/ThirdPersonBP/Blueprints/ThirdPersonCharacter.SetCharacterScaleEvent` _asthird_person_character)
  (`KismetSystemLibrary.Delay` 0.05)
  (set `/Game/ThirdPersonBP/Blueprints/ThirdPersonCharacter.skorost` 0.0 _asthird_person_character)
  (bind _returnvalue (`|CreateWidget` "/Game/Kirill/W_CutScene.W_CutScene_C" null _media_player "/Game/Kirill/green_lights.green_lights"))
  (`UserWidget.AddToViewport` _returnvalue 0)
  (add `MediaPlayer.OnEndReached` _media_player (delegate `Event_Video`))
  (bind _asbp_game_instanse (cast `/Game/Kirill/BP_game_instanse` (`GameplayStatics.GetGameInstance`)))
  (set `/Game/Kirill/BP_game_instanse.start_game?` false _asbp_game_instanse)
  (`KismetSystemLibrary.Delay` 2.0)
  (`GameplayStatics.OpenLevel` "ThirdPersonExampleMap"))

(event `Event_Video`
  (`Widget.RemoveFromParent` (stale `self.Box.OnComponentBeginOverlap` _returnvalue)))

(fn `UserConstructionScript`)