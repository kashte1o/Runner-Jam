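; A pipe module lever actor (Rychag) that turns when something enters its trigger box.
; The Box overlap event plays a timeline whose track drives a lerp of the lever's relative yaw toward 180 degrees, keeping roll and pitch.
; The lerp starts from the current yaw each update rather than a stored start value, and nothing in the graph reverses the motion or filters the overlapping actor.
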(event `self.Box.OnComponentBeginOverlap`
  (params (OverlappedComponent :type "PrimitiveComponent Object Reference") (OtherActor :type "Actor Object Reference") (OtherComp :type "PrimitiveComponent Object Reference") (OtherBodyIndex :type Integer) (bFromSweep :type Boolean) (SweepResult :type "HitResult Structure (by ref)"))
  (bind _rychag (`self.Rychag`))
  (bind (_relativerotation_roll _relativerotation_pitch _relativerotation_yaw) (`KismetMathLibrary.BreakRotator` (`SceneComponent.RelativeRotation` _rychag)))
  (bind (_direction _newtrack_0) (`Timeline|Timeline_01`)
    (:`Update`
      (`SceneComponent.K2_SetRelativeRotation` _rychag (`KismetMathLibrary.MakeRotator` _relativerotation_roll _relativerotation_pitch (`KismetMathLibrary.Lerp` _relativerotation_yaw 180.0 _newtrack_0)) false false))))

(fn `UserConstructionScript`
  (`parent.UserConstructionScript`))