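; BP_StartRoom is the start room actor, containing a clickable start button that animates when pressed.
; On BeginPlay it reads the StartGame flag from BP_game_instanse and destroys itself if the flag is false.
; Clicking and releasing the button drive two timelines that lerp its relative X and Z to pressed and, after a short delay, raised positions.
; The button only animates here, and its sound call is unconnected.
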(event `self.ReceiveBeginPlay`
  (bind _asbp_game_instanse (cast `/Game/Kirill/BP_game_instanse` (`GameplayStatics.GetGameInstance`)))
  (if (not (`/Game/Kirill/BP_game_instanse.start_game?` _asbp_game_instanse))
    (`self.K2_DestroyActor`)))

(event `self.Start_Button.OnClicked`
  (params (TouchedComponent :type "PrimitiveComponent Object Reference") (ButtonPressed :type "Key Structure"))
  (bind _start_button (`self.Start_Button`))
  (bind (_relativelocation_x _relativelocation_y _relativelocation_z) (`KismetMathLibrary.BreakVector` (`SceneComponent.RelativeLocation` _start_button)))
  (bind (_direction _newtrack_0) (`Timeline|Button_Timeline`)
    (:`Update`
      (set `self.X` _relativelocation_x)
      (set `self.Z` _relativelocation_z)
      (`SceneComponent.K2_SetRelativeLocation` _start_button (`KismetMathLibrary.MakeVector` (`KismetMathLibrary.Lerp` (`self.X`) 13.174833 _newtrack_0) _relativelocation_y (`KismetMathLibrary.Lerp` (`self.Z`) -25.375011 _newtrack_0)) false false))))

(event `self.Start_Button.OnReleased`
  (params (TouchedComponent :type "PrimitiveComponent Object Reference") (ButtonReleased :type "Key Structure"))
  (bind _start_button (`self.Start_Button`))
  (bind (_relativelocation_x _relativelocation_y _relativelocation_z) (`KismetMathLibrary.BreakVector` (`SceneComponent.RelativeLocation` _start_button)))
  (`KismetSystemLibrary.Delay` 0.5)
  (bind (_direction _newtrack_0) (`Timeline|Timeline_0`)
    (:`Update`
      (`SceneComponent.K2_SetRelativeLocation` _start_button (`KismetMathLibrary.MakeVector` (`KismetMathLibrary.Lerp` _relativelocation_x 14.293219 _newtrack_0) _relativelocation_y (`KismetMathLibrary.Lerp` _relativelocation_z -23.716938 _newtrack_0)) false false))))

(fn `UserConstructionScript`)