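; BP_object1 is an unfinished actor Blueprint that rolls a random number on BeginPlay, with no visible effect in the game.
; The random float is truncated to an integer and converted to a string for a switch that has no wired branches.
; An unconnected node would set the Cube component's mesh to SM_Rychag_V01, but it never runs.
; Overlap and Tick events are disabled, and the construction script only calls its parent.
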(event `self.ReceiveBeginPlay`
  (`parent.ReceiveBeginPlay`)
  (bind _output_get (set `self.i` (`KismetMathLibrary.FTrunc` (`KismetMathLibrary.RandomFloatInRange` 1.0 5.0))))
  (switch `string` (`KismetStringLibrary.Conv_IntToString` _output_get)))

(fn `UserConstructionScript`
  (`parent.UserConstructionScript`))